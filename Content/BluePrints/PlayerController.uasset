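; Player pawn Blueprint, named PlayerController, that toggles the Boids menu.
; On BeginPlay it casts its controller and adds the Enhanced Input mapping context for the menu.
; The IA_Menu action creates a new BoidsMenu widget if none is open, switches to UI-only input and shows the cursor.
; Because input is then UI-only, a separate CloseMenu event removes the widget and restores game input and cursor state.
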(event Custom|Close%20Menu
  (bind _returnvalue (Game|GetPlayerController 0))
  ;[1 1 1] Closes menu
  (if (Variables|Default|GetMenuOpen)
    (Widget|RemovefromParent (Variables|Default|GetMenu))
    (Input|SetInputModeGameOnly _returnvalue false)
    (bind _output_get (Variables|Default|SetMenuOpen false))
    (Variables|/Script/Engine.PlayerController|SetbShowMouseCursor _returnvalue _output_get)))

(event Input|EnhancedActionEvents|EnhancedInputActionIA_Menu
  (params (ActionValue :type Boolean) (ElapsedSeconds :type Float%20%28double-precision%29) (TriggeredSeconds :type Float%20%28double-precision%29) (InputAction :type Input%20Action%20Object%20Reference :default "/Game/Input/IA_Menu.IA_Menu"))
  (bind _returnvalue (Game|GetPlayerController 0))
  ;[1 1 1] Opens menu when p is pressed
  (if (not (Variables|Default|GetMenuOpen))
    (bind _returnvalue_2 (UserInterface|CreateWidget "/Game/BluePrints/BoidsMenu.BoidsMenu_C" _returnvalue))
    (bind _output_get (Variables|Default|SetMenu _returnvalue_2))
    (UserInterface|Viewport|AddtoViewport _output_get 0)
    (Input|SetInputModeUIOnly _returnvalue _output_get "DoNotLock" false)
    (bind _output_get_2 (Variables|Default|SetMenuOpen true))
    (Variables|/Script/Engine.PlayerController|SetbShowMouseCursor _returnvalue _output_get_2)))

(event EventBeginPlay
  ;[1 1 1] Adds input mapping for menu
  (bind _asplayer_controller (Utilities|Casting|CastToPlayerController (Pawn|GetController)))
  (Input|AddMappingContext (PlayerController|LocalPlayerSubsystems|GetEnhancedInputLocalPlayerSubsystem _asplayer_controller) "/Game/Input/InputActions.InputActions" 0 "(bIgnoreAllPressedKeysUntilRelease=True,bForceImmediately=False,bNotifyUserSettings=False)"))

(fn ConstructionScript)